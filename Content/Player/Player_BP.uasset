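; Player character Blueprint that handles input, HUD setup and game-over conditions.
; On BeginPlay in the Graybox level, it adds the default Enhanced Input mapping, shows PlayerUI and sets game-only input.
; Movement follows fixed world axes, and jump input also sets an IsJumping flag.
; RemoveGoober counts down CurrentGoobers, loading the main menu at zero, as does capsule overlap with DEATH; the Game_Success overlap has no action.
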(event `self.ReceiveBeginPlay`
  (bind _returnvalue (`GameplayStatics.GetPlayerController` 0))
  (bind _returnvalue_2 (pcsubsystem `EnhancedInputLocalPlayerSubsystem` _returnvalue))
  ;[1 1 1] HUD/Input Mapping
  (bind _returnvalue_3 (`GameplayStatics.GetCurrentLevelName` true))
  (if (== _returnvalue_3 "Graybox")
    (`/Engine/EditorBlueprintResources/StandardMacros.IsValid` _returnvalue_2
      (:`Is Valid`
        (`EnhancedInputSubsystemInterface.AddMappingContext` _returnvalue_2 "/Game/Player_Input/Input_Controls_Default.Input_Controls_Default" 0 (struct))
        (bind _returnvalue_4 (`|CreateWidget` "/Game/UI/PlayerUI.PlayerUI_C" _returnvalue))
        (`UserWidget.AddToViewport` _returnvalue_4 0)
        (`WidgetBlueprintLibrary.SetInputMode_GameOnly` _returnvalue)))))

(event `EnhancedInput|/Game/Player_Input/Input_Movement`
  (params (ActionValue :type "Vector2D Structure") (ElapsedSeconds :type "Float (double-precision)") (TriggeredSeconds :type "Float (double-precision)") (InputAction :type "InputAction Object Reference" :default "/Game/Player_Input/Input_Movement.Input_Movement"))
  ;[1 1 1] Player Movement
  (:`Triggered`
    (`self.AddMovementInput` (2.0 0.0 0.0) ActionValue_X true) ; Left/Right
    (`self.AddMovementInput` (0.0 -2.0 0.0) ActionValue_Y true) ; Up/Down
  ))

(event `EnhancedInput|/Game/Player_Input/Input_Jump`
  (params (ActionValue :type Boolean) (ElapsedSeconds :type "Float (double-precision)") (TriggeredSeconds :type "Float (double-precision)") (InputAction :type "InputAction Object Reference" :default "/Game/Player_Input/Input_Jump.Input_Jump"))
  ;[1 1 1] Jumping
  (:`Triggered`
    (set `self.IsJumping` true)
    (`self.Jump`))
  (:`Completed`
    (set `self.IsJumping` false)
    (`self.StopJumping`)))

(event `Remove Goober`
  (bind _current_goobers (`self.Current_Goobers`))
  ;[1 1 1] Game End
  (bind _result (`/Engine/EditorBlueprintResources/StandardMacros.DecrementFloat` _current_goobers)
    (:`  `
      (`KismetSystemLibrary.PrintString` (`KismetStringLibrary.Conv_DoubleToString` _current_goobers))
      (if (<= _result 0.0)
        (`GameplayStatics.OpenLevel` "MainMenu_Level" :!label _label)))))

(event `self.CapsuleComponent.OnComponentBeginOverlap`
  (params (OverlappedComponent :type "PrimitiveComponent Object Reference") (OtherActor :type "Actor Object Reference") (OtherComp :type "PrimitiveComponent Object Reference") (OtherBodyIndex :type Integer) (bFromSweep :type Boolean) (SweepResult :type "HitResult Structure (by ref)"))
  ;[1 1 1] Game End
  (bind _asdeath (cast `/Game/Player/DEATH` OtherActor)
    (:`then`
      (`/Engine/EditorBlueprintResources/StandardMacros.IsValid` _asdeath
        (:`Is Valid`
          (goto _label))))
    (:`CastFailed`
      (cast `/Game/Game_Success` OtherActor))))

(fn `UserConstructionScript`)