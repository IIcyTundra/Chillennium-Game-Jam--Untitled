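; PlayerAI_BP is an AI follower character, a "Goober", that trails the player and can die in hazards.
; Each tick it issues AI Move To toward the player and jumps when a downward trace ahead finds no ground.
; It also applies Input_Movement on fixed world axes.
; Overlapping a Do_Dmg actor starts a delayed damage loop that destroys it at zero HP and decrements the player's CurrentGoobers.
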(event `EnhancedInput|/Game/Player_Input/Input_Movement`
  (params (ActionValue :type "Vector2D Structure") (ElapsedSeconds :type "Float (double-precision)") (TriggeredSeconds :type "Float (double-precision)") (InputAction :type "InputAction Object Reference" :default "/Game/Player_Input/Input_Movement.Input_Movement"))
  ;[1 1 1] Player Movement
  (:`Triggered`
    (`self.AddMovementInput` (1.0 0.0 0.0) ActionValue_X true) ; Left/Right
    (`self.AddMovementInput` (0.0 -1.0 0.0) ActionValue_Y true) ; Up/Down
  ))

(event `self.ReceiveTick`
  (params (DeltaSeconds :type "Float (single-precision)"))
  (bind _returnvalue (+ (`self.K2_GetActorLocation`) (* (`self.GetActorForwardVector`) 100.0)))
  ;[1 1 1] Follow Player
  (bind _asplayer_bp (cast `/Game/Player/Player_BP` (`GameplayStatics.GetPlayerCharacter` 0)))
  (`/Engine/EditorBlueprintResources/StandardMacros.IsValid` _asplayer_bp
    (:`Is Valid`
      (`|AIMoveTo` self (0.0 0.0 0.0) _asplayer_bp 5.0 true
        (:`then`
          (bind (_outhit _returnvalue_2) (`KismetSystemLibrary.LineTraceSingle` :`Start` _returnvalue :`End` (- _returnvalue (0.0 0.0 50.0)) :`TraceChannel` "TraceTypeQuery1" :`DrawDebugType` "ForOneFrame"))
          (if _returnvalue_2
            _
            (elif (not (`NavMovementComponent.IsFalling` (`self.CharacterMovement`)))
              (`self.Jump`))))))))

(event `self.CapsuleComponent.OnComponentBeginOverlap`
  (params (OverlappedComponent :type "PrimitiveComponent Object Reference") (OtherActor :type "Actor Object Reference") (OtherComp :type "PrimitiveComponent Object Reference") (OtherBodyIndex :type Integer) (bFromSweep :type Boolean) (SweepResult :type "HitResult Structure (by ref)"))
  ;[1 1 1] Do damage on enter hazard
  (bind _asdo_dmg (cast `/Game/Gameplay_Elements/Do_Dmg` OtherActor))
  (`/Engine/EditorBlueprintResources/StandardMacros.IsValid` _asdo_dmg
    (:`Is Valid`
      (set `self.In bound` true)
      (bind _output_get (set `self.GooberHP` (- (`self.GooberHP`) 5.0) :!label _label))
      (`KismetSystemLibrary.PrintString` (`KismetStringLibrary.Conv_DoubleToString` _output_get))
      (`KismetSystemLibrary.Delay` 0.6)
      (if (`self.In bound`)
        (if (<= _output_get 0.0)
          (`self.K2_DestroyActor`)
          (bind _asplayer_bp (cast `/Game/Player/Player_BP` (`GameplayStatics.GetPlayerCharacter` 0)))
          (set `/Game/Player/Player_BP.Current_Goobers` (- (`/Game/Player/Player_BP.Current_Goobers` _asplayer_bp) 1.0) _asplayer_bp)
          (else
            (goto _label)))))))

(fn `UserConstructionScript`)